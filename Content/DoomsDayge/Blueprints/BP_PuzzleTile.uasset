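; BP_PuzzleTile is a single puzzle tile built on a cube mesh whose material is configured per instance.
; The Construction Script creates a dynamic instance of the puzzle material on the cube and stores it.
; It passes the tile's U, V and Size variables to the material as scalar parameters, apparently selecting that tile's portion of the puzzle image.
; The Interaction event is an empty stub.
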(event EventInteraction)

(fn ConstructionScript
  (bind _returnvalue (Rendering|Material|CreateDynamicMaterialInstance (Variables|Default|GetCube) 0 "/Game/DoomsDayge/Materials/PuzzleMAT.PuzzleMAT" "None" :!class /Script/Engine.PrimitiveComponent))
  (bind _output_get (Variables|Default|SetPuzzleMID _returnvalue))
  (Rendering|Material|SetScalarParameterValue _output_get "CustomU" (Math|Conversions|ToFloat(Integer) (Variables|Default|GetU)) :!class /Script/Engine.MaterialInstanceDynamic)
  (Rendering|Material|SetScalarParameterValue _output_get "CustomV" (Math|Conversions|ToFloat(Integer) (Variables|Default|GetV)) :!class /Script/Engine.MaterialInstanceDynamic)
  (Rendering|Material|SetScalarParameterValue _output_get "Size" (Math|Conversions|ToFloat(Integer) (Variables|Default|GetSize)) :!class /Script/Engine.MaterialInstanceDynamic))