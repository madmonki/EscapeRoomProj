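; Rotatable picture frame for a puzzle that is solved when every frame of this class sits at its answer position.
; Interaction plays a sound and a timeline that pitches the frame 90 degrees, cycles its position through four steps and updates its Finalized flag.
; Each instance gathers all frames at BeginPlay and polls their flags on a looping timer.
; Once all are finalized, it stops its timer and fires the puzzle-completed dispatcher.
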(event Custom|RotatePainting
  (if (not (Variables|Default|GetFrameMoving))
    (bind _result (Math|Integer|IncrementInt (Variables|Default|GetFramePosition))
      (:%20%20
        (Variables|Default|SetFramePosition (Math|Integer|%(Integer) _result 4))
        (Variables|Default|SetFrameMoving true)
        (Audio|PlaySound2D "/Game/DoomsDayge/Sound/327555__damianminnie__moving-object-heavy-object-moved-accros-surface.327555__damianminnie__moving-object-heavy-object-moved-accros-surface" 1.0 1.0 0.0 0 0)
        (bind _rotation (Timeline|PaintingRotation PlayFromStart)
          (:Update
            (Transformation|SetRelativeRotation (Variables|Default|GetPictureFrame) (Math|Rotator|MakeRotator 0.0 (Math|Float|Lerp (.pitch (Variables|Default|GetStartingRotationFrame)) (+ (.pitch (Variables|Default|GetStartingRotationFrame)) 9e+01) _rotation) 0.0) false false))
          (:Finished
            (Variables|Default|SetStartingRotationFrame (Math|Rotator|MakeRotator 0.0 (Math|Float|Lerp (.pitch (Variables|Default|GetStartingRotationFrame)) (+ (.pitch (Variables|Default|GetStartingRotationFrame)) 9e+01) _rotation) 0.0))
            (Variables|Default|SetFrameMoving false)))))))

(event Custom|PuzzleCheck
  (for _array_element (Variables|Default|GetAllPictureFrames)
    (if (not (Variables|BP_PictureFrame_PuzzleMaster_C|GetFinalized _array_element))
      (Variables|Default|SetPuzzleSolved false)))
  (if (Variables|Default|GetPuzzleSolved)
    (Utilities|Time|ClearandInvalidateTimerbyHandle (stale EventBeginPlay _returnvalue))
    (Default|CallEVDPuzzleCompleted)
    (else
      (Variables|Default|SetPuzzleSolved true))))

(event EventInteraction
  (CallFunction|RotatePainting)
  (if (== (Variables|Default|GetFramePosition) (Variables|Default|GetPuzzleAnswer))
    (Variables|Default|SetFinalized true)
    (else
      (Variables|Default|SetFinalized false))))

(event EventBeginPlay
  (Variables|Default|SetStartingRotationFrame (Variables|/Script/Engine.SceneComponent|GetRelativeRotation (Variables|Default|GetPictureFrame)))
  (bind _outactors (Actor|GetAllActorsOfClass "BP_PictureFrame_PuzzleMaster_C"))
  (Variables|Default|SetAllPictureFrames _outactors)
  (bind _returnvalue (Utilities|Time|SetTimerbyEvent (delegate Custom|PuzzleCheck) 1.0 true))
  (if (== (Variables|Default|GetFramePosition) (Variables|Default|GetPuzzleAnswer))
    (Variables|Default|SetFinalized true)
    (else
      (Variables|Default|SetFinalized false))))

(fn ConstructionScript
  (|CallParentFunction))