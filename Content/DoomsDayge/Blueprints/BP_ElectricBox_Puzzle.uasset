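; Electric box puzzle where the player clicks four switches to find the correct on/off combination and earn the key to the next level.
; Interaction blends the view to the box, freezes the player and enables cursor clicks; IA_Back or solving restores control.
; Each switch toggles a rotation timeline, whose completion shifts two needles by per-switch offsets and checks the answer.
; Only switches 1 and 3 on solves it, spawning BP_KeyToNextLevel at BP_LevelInfo's location.
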(event OnClicked(switch0)
  (params (TouchedComponent :type Primitive%20Component%20Object%20Reference) (ButtonPressed :type Key%20Structure :default "None"))
  (bind _switch0 (Variables|Default|Getswitch0))
  (bind _relativerotation (Variables|/Script/Engine.SceneComponent|GetRelativeRotation _switch0))
  (Audio|PlaySound2D "/Game/DoomsDayge/Sound/649878__hydrocityharry__light-switch.649878__hydrocityharry__light-switch" 1.0 1.0 0.0 0 0)
  (Utilities|FlowControl|FlipFlop
    (:A
      (Variables|Default|SetSwitch0_On true)
      (bind _newtrack_0 (Timeline|SwitchRotate0 Play)
        (:Update
          (Transformation|SetRelativeRotation _switch0 (Math|Rotator|MakeRotator _newtrack_0 (.pitch _relativerotation) (.yaw _relativerotation)) false false))
        (:Finished
          (CallFunction|Switch00)
          (CallFunction|AnswerCheck))))
    (:B
      (Variables|Default|SetSwitch0_On false)
      (Timeline|SwitchRotate0 Reverse))))

(event OnClicked(switch1)
  (params (TouchedComponent :type Primitive%20Component%20Object%20Reference) (ButtonPressed :type Key%20Structure :default "None"))
  (bind _switch1 (Variables|Default|Getswitch1))
  (bind _relativerotation (Variables|/Script/Engine.SceneComponent|GetRelativeRotation _switch1))
  (Audio|PlaySound2D "/Game/DoomsDayge/Sound/649878__hydrocityharry__light-switch.649878__hydrocityharry__light-switch" 1.0 1.0 0.0 0 0)
  (Utilities|FlowControl|FlipFlop
    (:A
      (Variables|Default|SetSwitch1_On true)
      (bind _newtrack_0 (Timeline|SwitchRotate1 Play)
        (:Update
          (Transformation|SetRelativeRotation _switch1 (Math|Rotator|MakeRotator _newtrack_0 (.pitch _relativerotation) (.yaw _relativerotation)) false false))
        (:Finished
          (CallFunction|Switch01)
          (CallFunction|AnswerCheck))))
    (:B
      (Variables|Default|SetSwitch1_On false)
      (Timeline|SwitchRotate1 Reverse))))

(event OnClicked(switch2)
  (params (TouchedComponent :type Primitive%20Component%20Object%20Reference) (ButtonPressed :type Key%20Structure :default "None"))
  (bind _switch2 (Variables|Default|Getswitch2))
  (bind _relativerotation (Variables|/Script/Engine.SceneComponent|GetRelativeRotation _switch2))
  (Audio|PlaySound2D "/Game/DoomsDayge/Sound/649878__hydrocityharry__light-switch.649878__hydrocityharry__light-switch" 1.0 1.0 0.0 0 0)
  (Utilities|FlowControl|FlipFlop
    (:A
      (Variables|Default|SetSwitch2_On true)
      (bind _newtrack_0 (Timeline|SwitchRotate2 Play)
        (:Update
          (Transformation|SetRelativeRotation _switch2 (Math|Rotator|MakeRotator _newtrack_0 (.pitch _relativerotation) (.yaw _relativerotation)) false false))
        (:Finished
          (CallFunction|Switch02)
          (CallFunction|AnswerCheck))))
    (:B
      (Variables|Default|SetSwitch2_On false)
      (Timeline|SwitchRotate2 Reverse))))

(event OnClicked(switch3)
  (params (TouchedComponent :type Primitive%20Component%20Object%20Reference) (ButtonPressed :type Key%20Structure :default "None"))
  (bind _switch3 (Variables|Default|Getswitch3))
  (bind _relativerotation (Variables|/Script/Engine.SceneComponent|GetRelativeRotation _switch3))
  (Audio|PlaySound2D "/Game/DoomsDayge/Sound/649878__hydrocityharry__light-switch.649878__hydrocityharry__light-switch" 1.0 1.0 0.0 0 0)
  (Utilities|FlowControl|FlipFlop
    (:A
      (Variables|Default|SetSwitch3_On true)
      (bind _newtrack_0 (Timeline|SwitchRotate3 Play)
        (:Update
          (Transformation|SetRelativeRotation _switch3 (Math|Rotator|MakeRotator _newtrack_0 (.pitch _relativerotation) (.yaw _relativerotation)) false false))
        (:Finished
          (CallFunction|Switch03)
          (CallFunction|AnswerCheck))))
    (:B
      (Variables|Default|SetSwitch3_On false)
      (Timeline|SwitchRotate3 Reverse))))

(event Custom|Switch03
  (bind _needle0 (Variables|Default|Getneedle0))
  (bind _needle0_2 (Variables|Default|Getneedle0))
  (bind _needle1 (Variables|Default|Getneedle1))
  (bind _needle1_2 (Variables|Default|Getneedle1))
  (if (Variables|Default|GetSwitch3_On)
    (Utilities|FlowControl|Sequence
      (:then_0
        (Components|MoveComponentTo _needle0_2 (Variables|/Script/Engine.SceneComponent|GetRelativeLocation _needle0_2) (Math|Rotator|MakeRotator 0.0 (+ (.pitch (Variables|Default|GetNeedle0_Rotation)) 0.0) (.yaw (Variables|Default|GetNeedle0_Rotation))) false false 0.2 false)
        (Variables|Default|SetNeedle0_Rotation (Math|Rotator|MakeRotator 0.0 (+ (.pitch (Variables|Default|GetNeedle0_Rotation)) 0.0) (.yaw (Variables|Default|GetNeedle0_Rotation)))))
      (:then_1
        (Components|MoveComponentTo _needle1_2 (Variables|/Script/Engine.SceneComponent|GetRelativeLocation _needle1_2) (Math|Rotator|MakeRotator 0.0 (+ (.pitch (Variables|Default|GetNeedle1_Rotation)) 15.0) (.yaw (Variables|Default|GetNeedle1_Rotation))) false false 0.2 false)
        (Variables|Default|SetNeedle1_Rotation (Math|Rotator|MakeRotator 0.0 (+ (.pitch (Variables|Default|GetNeedle1_Rotation)) 15.0) (.yaw (Variables|Default|GetNeedle1_Rotation))))))
    (else
      (Utilities|FlowControl|Sequence
        (:then_0
          (Components|MoveComponentTo _needle0 (Variables|/Script/Engine.SceneComponent|GetRelativeLocation _needle0) (Math|Rotator|MakeRotator 0.0 (+ (.pitch (Variables|Default|GetNeedle0_Rotation)) 0.0) (.yaw (Variables|Default|GetNeedle0_Rotation))) false false 0.2 false)
          (Variables|Default|SetNeedle0_Rotation (Math|Rotator|MakeRotator 0.0 (+ (.pitch (Variables|Default|GetNeedle0_Rotation)) 0.0) (.yaw (Variables|Default|GetNeedle0_Rotation)))))
        (:then_1
          (Components|MoveComponentTo _needle1 (Variables|/Script/Engine.SceneComponent|GetRelativeLocation _needle1) (Math|Rotator|MakeRotator 0.0 (+ (.pitch (Variables|Default|GetNeedle1_Rotation)) -15.0) (.yaw (Variables|Default|GetNeedle1_Rotation))) false false 0.2 false)
          (Variables|Default|SetNeedle1_Rotation (Math|Rotator|MakeRotator 0.0 (+ (.pitch (Variables|Default|GetNeedle1_Rotation)) -15.0) (.yaw (Variables|Default|GetNeedle1_Rotation)))))))))

(event Custom|Switch00
  (bind _needle0 (Variables|Default|Getneedle0))
  (bind _needle0_2 (Variables|Default|Getneedle0))
  (bind _needle1 (Variables|Default|Getneedle1))
  (bind _needle1_2 (Variables|Default|Getneedle1))
  (if (Variables|Default|GetSwitch0_On)
    (Utilities|FlowControl|Sequence
      (:then_0
        (Components|MoveComponentTo _needle0 (Variables|/Script/Engine.SceneComponent|GetRelativeLocation _needle0) (Math|Rotator|MakeRotator 0.0 (+ (.pitch (Variables|Default|GetNeedle0_Rotation)) 25.0) (.yaw (Variables|Default|GetNeedle0_Rotation))) false false 0.2 false)
        (Variables|Default|SetNeedle0_Rotation (Math|Rotator|MakeRotator 0.0 (+ (.pitch (Variables|Default|GetNeedle0_Rotation)) 25.0) (.yaw (Variables|Default|GetNeedle0_Rotation)))))
      (:then_1
        (Components|MoveComponentTo _needle1 (Variables|/Script/Engine.SceneComponent|GetRelativeLocation _needle1) (Math|Rotator|MakeRotator 0.0 (+ (.pitch (Variables|Default|GetNeedle1_Rotation)) 1e+01) (.yaw (Variables|Default|GetNeedle1_Rotation))) false false 0.2 false)
        (Variables|Default|SetNeedle1_Rotation (Math|Rotator|MakeRotator 0.0 (+ (.pitch (Variables|Default|GetNeedle1_Rotation)) 1e+01) (.yaw (Variables|Default|GetNeedle1_Rotation))))))
    (else
      (Utilities|FlowControl|Sequence
        (:then_0
          (Components|MoveComponentTo _needle0_2 (Variables|/Script/Engine.SceneComponent|GetRelativeLocation _needle0_2) (Math|Rotator|MakeRotator 0.0 (+ (.pitch (Variables|Default|GetNeedle0_Rotation)) -25.0) (.yaw (Variables|Default|GetNeedle0_Rotation))) false false 0.2 false)
          (Variables|Default|SetNeedle0_Rotation (Math|Rotator|MakeRotator 0.0 (+ (.pitch (Variables|Default|GetNeedle0_Rotation)) -25.0) (.yaw (Variables|Default|GetNeedle0_Rotation)))))
        (:then_1
          (Components|MoveComponentTo _needle1_2 (Variables|/Script/Engine.SceneComponent|GetRelativeLocation _needle1_2) (Math|Rotator|MakeRotator 0.0 (+ (.pitch (Variables|Default|GetNeedle1_Rotation)) -1e+01) (.yaw (Variables|Default|GetNeedle1_Rotation))) false false 0.2 false)
          (Variables|Default|SetNeedle1_Rotation (Math|Rotator|MakeRotator 0.0 (+ (.pitch (Variables|Default|GetNeedle1_Rotation)) -1e+01) (.yaw (Variables|Default|GetNeedle1_Rotation)))))))))

(event Custom|GetAway
  (bind _returnvalue (Game|GetPlayerController 0))
  (bind _playerref (Variables|Default|GetPlayerRef))
  (Game|Player|SetViewTargetwithBlend (Game|GetPlayerController 0) (Variables|Default|GetPlayerRef) 0.5 "VTBlend_Linear" 0.0 false)
  (Variables|/Script/Engine.PlayerController|SetbEnableClickEvents _returnvalue false)
  (Variables|/Script/Engine.PlayerController|SetbShowMouseCursor _returnvalue false)
  (Pawn|Components|CharacterMovement|SetMovementMode (Variables|/Script/Engine.Character|GetCharacterMovement _playerref) "MOVE_Walking" 0)
  (Variables|/Game/FirstPerson/Blueprints/BP_FirstPersonCharacter.BP_FirstPersonCharacter_C|SetAllowLook _playerref true)
  (Widget|SetVisibility (Variables|/Game/FirstPerson/Blueprints/BP_FirstPersonCharacter.BP_FirstPersonCharacter_C|GetCHVar _playerref) "Visible")
  (Class|GameplayStatics|SetViewportMouseCaptureMode "CapturePermanently"))

(event Custom|Switch01
  (bind _needle0 (Variables|Default|Getneedle0))
  (bind _needle0_2 (Variables|Default|Getneedle0))
  (bind _needle1 (Variables|Default|Getneedle1))
  (bind _needle1_2 (Variables|Default|Getneedle1))
  (if (Variables|Default|GetSwitch1_On)
    (Utilities|FlowControl|Sequence
      (:then_0
        (Components|MoveComponentTo _needle0 (Variables|/Script/Engine.SceneComponent|GetRelativeLocation _needle0) (Math|Rotator|MakeRotator 0.0 (+ (.pitch (Variables|Default|GetNeedle0_Rotation)) 3e+01) (.yaw (Variables|Default|GetNeedle0_Rotation))) false false 0.2 false)
        (Variables|Default|SetNeedle0_Rotation (Math|Rotator|MakeRotator 0.0 (+ (.pitch (Variables|Default|GetNeedle0_Rotation)) 3e+01) (.yaw (Variables|Default|GetNeedle0_Rotation)))))
      (:then_1
        (Components|MoveComponentTo _needle1 (Variables|/Script/Engine.SceneComponent|GetRelativeLocation _needle1) (Math|Rotator|MakeRotator 0.0 (+ (.pitch (Variables|Default|GetNeedle1_Rotation)) 45.0) (.yaw (Variables|Default|GetNeedle1_Rotation))) false false 0.2 false)
        (Variables|Default|SetNeedle1_Rotation (Math|Rotator|MakeRotator 0.0 (+ (.pitch (Variables|Default|GetNeedle1_Rotation)) 45.0) (.yaw (Variables|Default|GetNeedle1_Rotation))))))
    (else
      (Utilities|FlowControl|Sequence
        (:then_0
          (Components|MoveComponentTo _needle0_2 (Variables|/Script/Engine.SceneComponent|GetRelativeLocation _needle0_2) (Math|Rotator|MakeRotator 0.0 (+ (.pitch (Variables|Default|GetNeedle0_Rotation)) -3e+01) (.yaw (Variables|Default|GetNeedle0_Rotation))) false false 0.2 false)
          (Variables|Default|SetNeedle0_Rotation (Math|Rotator|MakeRotator 0.0 (+ (.pitch (Variables|Default|GetNeedle0_Rotation)) -3e+01) (.yaw (Variables|Default|GetNeedle0_Rotation)))))
        (:then_1
          (Components|MoveComponentTo _needle1_2 (Variables|/Script/Engine.SceneComponent|GetRelativeLocation _needle1_2) (Math|Rotator|MakeRotator 0.0 (+ (.pitch (Variables|Default|GetNeedle1_Rotation)) -45.0) (.yaw (Variables|Default|GetNeedle1_Rotation))) false false 0.2 false)
          (Variables|Default|SetNeedle1_Rotation (Math|Rotator|MakeRotator 0.0 (+ (.pitch (Variables|Default|GetNeedle1_Rotation)) -45.0) (.yaw (Variables|Default|GetNeedle1_Rotation)))))))))

(event Custom|Switch02
  (bind _needle0 (Variables|Default|Getneedle0))
  (bind _needle0_2 (Variables|Default|Getneedle0))
  (bind _needle1 (Variables|Default|Getneedle1))
  (bind _needle1_2 (Variables|Default|Getneedle1))
  (if (Variables|Default|GetSwitch2_On)
    (Utilities|FlowControl|Sequence
      (:then_0
        (Components|MoveComponentTo _needle0 (Variables|/Script/Engine.SceneComponent|GetRelativeLocation _needle0) (Math|Rotator|MakeRotator 0.0 (+ (.pitch (Variables|Default|GetNeedle0_Rotation)) 2e+01) (.yaw (Variables|Default|GetNeedle0_Rotation))) false false 0.2 false)
        (Variables|Default|SetNeedle0_Rotation (Math|Rotator|MakeRotator 0.0 (+ (.pitch (Variables|Default|GetNeedle0_Rotation)) 2e+01) (.yaw (Variables|Default|GetNeedle0_Rotation)))))
      (:then_1
        (Components|MoveComponentTo _needle1 (Variables|/Script/Engine.SceneComponent|GetRelativeLocation _needle1) (Math|Rotator|MakeRotator 0.0 (+ (.pitch (Variables|Default|GetNeedle1_Rotation)) 5.0) (.yaw (Variables|Default|GetNeedle1_Rotation))) false false 0.2 false)
        (Variables|Default|SetNeedle1_Rotation (Math|Rotator|MakeRotator 0.0 (+ (.pitch (Variables|Default|GetNeedle1_Rotation)) 5.0) (.yaw (Variables|Default|GetNeedle1_Rotation))))))
    (else
      (Utilities|FlowControl|Sequence
        (:then_0
          (Components|MoveComponentTo _needle0_2 (Variables|/Script/Engine.SceneComponent|GetRelativeLocation _needle0_2) (Math|Rotator|MakeRotator 0.0 (+ (.pitch (Variables|Default|GetNeedle0_Rotation)) -2e+01) (.yaw (Variables|Default|GetNeedle0_Rotation))) false false 0.2 false)
          (Variables|Default|SetNeedle0_Rotation (Math|Rotator|MakeRotator 0.0 (+ (.pitch (Variables|Default|GetNeedle0_Rotation)) -2e+01) (.yaw (Variables|Default|GetNeedle0_Rotation)))))
        (:then_1
          (Components|MoveComponentTo _needle1_2 (Variables|/Script/Engine.SceneComponent|GetRelativeLocation _needle1_2) (Math|Rotator|MakeRotator 0.0 (+ (.pitch (Variables|Default|GetNeedle1_Rotation)) -5.0) (.yaw (Variables|Default|GetNeedle1_Rotation))) false false 0.2 false)
          (Variables|Default|SetNeedle1_Rotation (Math|Rotator|MakeRotator 0.0 (+ (.pitch (Variables|Default|GetNeedle1_Rotation)) -5.0) (.yaw (Variables|Default|GetNeedle1_Rotation)))))))))

(event Custom|AnswerCheck
  (if (and (Variables|Default|GetSwitch1_On) (Variables|Default|GetSwitch3_On))
    (if (not (Variables|Default|GetSwitch0_On))
      (if (not (Variables|Default|GetSwitch2_On))
        (Variables|Default|SetPuzzleSolved true)
        (CallFunction|GetAway)
        (Development|PrintString "Puzzle Solved")
        (bind _returnvalue (Actor|GetActorOfClass "/Game/DoomsDayge/Blueprints/BP_LevelInfo.BP_LevelInfo_C"))
        (Game|SpawnActorfromClass "/Game/DoomsDayge/Blueprints/BP_KeyToNextLevel.BP_KeyToNextLevel_C" (Math|Transform|MakeTransform (.location (Transformation|GetActorTransform _returnvalue)) "0.000000,0.000000,80.000000" "1.000000,1.000000,1.000000") "Undefined" "MultiplyWithRoot" 0 0)))))

(event Input|EnhancedActionEvents|EnhancedInputActionIA_Back
  (params (ActionValue :type Boolean) (ElapsedSeconds :type Float%20%28double-precision%29) (TriggeredSeconds :type Float%20%28double-precision%29) (InputAction :type Input%20Action%20Object%20Reference :default "/Game/DoomsDayge/Inputs/IA_Back.IA_Back"))
  (:Started
    (CallFunction|GetAway)))

(event EventBeginPlay
  (|CallParentFunction)
  (Input|EnableInput (Game|GetPlayerController 0))
  (Variables|Default|SetNeedle0_Rotation (Variables|/Script/Engine.SceneComponent|GetRelativeRotation (Variables|Default|Getneedle0)))
  (Variables|Default|SetNeedle1_Rotation (Variables|/Script/Engine.SceneComponent|GetRelativeRotation (Variables|Default|Getneedle1))))

(event EventInteraction
  (bind _returnvalue (Game|GetPlayerController 0))
  (bind _playerref (Variables|Default|GetPlayerRef))
  (if (not (Variables|Default|GetPuzzleSolved))
    (Game|Player|SetViewTargetwithBlend (Game|GetPlayerController 0) self 0.5 "VTBlend_Linear" 0.0 false)
    (Variables|/Script/Engine.PlayerController|SetbEnableClickEvents _returnvalue true)
    (Variables|/Script/Engine.PlayerController|SetbShowMouseCursor _returnvalue true)
    (Pawn|Components|CharacterMovement|DisableMovement (Variables|/Script/Engine.Character|GetCharacterMovement _playerref))
    (Variables|/Game/FirstPerson/Blueprints/BP_FirstPersonCharacter.BP_FirstPersonCharacter_C|SetAllowLook _playerref false)
    (Widget|SetVisibility (Variables|/Game/FirstPerson/Blueprints/BP_FirstPersonCharacter.BP_FirstPersonCharacter_C|GetCHVar _playerref) "Hidden")
    (Class|GameplayStatics|SetViewportMouseCaptureMode "CaptureDuringMouseDown")))

(fn ConstructionScript
  (|CallParentFunction))