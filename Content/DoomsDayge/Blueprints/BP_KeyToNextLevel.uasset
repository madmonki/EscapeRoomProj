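; Key actor for progressing to the next level, with logic here that only handles its drop sound.
; BeginPlay and the Dropkeysound event store the actor's current height as a baseline.
; When InspectMesh hits something at least 20 units below that baseline, SoundFX plays.
; Every hit resets the baseline to the mesh's current height, so small bumps and upward moves stay silent.
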(event OnComponentHit(InspectMesh)
  (params (HitComponent :type Primitive%20Component%20Object%20Reference) (OtherActor :type Actor%20Object%20Reference) (OtherComp :type Primitive%20Component%20Object%20Reference) (NormalImpulse :type Vector :default "0, 0, 0") (Hit :type Hit%20Result%20Structure%20%28by%20ref%29))
  (bind _returnvalue (Transformation|GetWorldLocation HitComponent))
  (if (>= (- (Variables|Default|GetInitialHeight) (.z _returnvalue)) 2e+01)
    (Variables|Default|SetInitialHeight (.z _returnvalue))
    (Audio|Components|Audio|Play (Variables|Default|GetSoundFX) 0.0)
    (else
      (Variables|Default|SetInitialHeight (.z _returnvalue)))))

(event EventBeginPlay
  (Variables|Default|SetInitialHeight (.z (Transformation|GetActorLocation))))

(event EventDropkeysound
  (Variables|Default|SetInitialHeight (.z (Transformation|GetActorLocation))))

(fn ConstructionScript
  (|CallParentFunction))