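; BP_Stand is one coloured button stand in a Simon-style memory game, reporting interactions to its main Simon actor during the player's turn with its Index.
; The construction script creates a dynamic material on the capsule tinted with the stand's Color.
; PlayNote plays a press cue and pulses emissive Intensity for half a second, while PlayError plays a failure cue and flashes red before restoring the colour.
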(event Custom|PlayError
  (bind _audio (Variables|Default|GetAudio))
  (Audio|Components|Audio|SetSound _audio "/Game/DoomsDayge/Sound/failure_Cue.failure_Cue")
  (Audio|Components|Audio|Play _audio 0.0)
  (Rendering|Material|SetVectorParameterValue (Variables|Default|GetDynMat) "Color" "(R=1.000000,G=0.000000,B=0.000000,A=1.000000)" :!class /Script/Engine.MaterialInstanceDynamic)
  (Rendering|Material|SetScalarParameterValue (Variables|Default|GetDynMat) "Intensity" 2.5 :!class /Script/Engine.MaterialInstanceDynamic)
  (Utilities|FlowControl|Delay 0.5)
  (Rendering|Material|SetScalarParameterValue (Variables|Default|GetDynMat) "Intensity" 0.0 :!class /Script/Engine.MaterialInstanceDynamic)
  (Rendering|Material|SetVectorParameterValue (Variables|Default|GetDynMat) "Color" (Variables|Default|GetColor) :!class /Script/Engine.MaterialInstanceDynamic))

(event Custom|PlayNote
  (bind _audio (Variables|Default|GetAudio))
  (Audio|Components|Audio|SetSound _audio "/Game/DoomsDayge/Sound/button-press_Cue.button-press_Cue")
  (Audio|Components|Audio|Play _audio 0.0)
  (Rendering|Material|SetScalarParameterValue (Variables|Default|GetDynMat) "Intensity" 2.5 :!class /Script/Engine.MaterialInstanceDynamic)
  (Utilities|FlowControl|Delay 0.5)
  (Rendering|Material|SetScalarParameterValue (Variables|Default|GetDynMat) "Intensity" 0.0 :!class /Script/Engine.MaterialInstanceDynamic))

(event EventBeginPlay
  (Audio|Components|Audio|SetSound (Variables|Default|GetAudio) (Variables|Default|GetPlayAudio)))

(event EventInteraction
  (bind _simonmain_ref (Variables|Default|GetSimonMain_Ref)
    (:then
      (if (Variables|/Game/DoomsDayge/Blueprints/BP_Simon.BP_Simon_C|GetisPlayersTurn _simonmain_ref)
        (Default|PlayerPlayedNote (Variables|Default|GetSimonMain_Ref) (Variables|Default|GetIndex))))
    (:else)))

(fn ConstructionScript
  (bind _returnvalue (Rendering|Material|CreateDynamicMaterialInstance (Variables|Default|GetCapsule) 1 "/Game/DoomsDayge/Materials/M_Colour.M_Colour" "None" :!class /Script/Engine.PrimitiveComponent))
  (bind _output_get (Variables|Default|SetDynMat _returnvalue))
  (Rendering|Material|SetVectorParameterValue _output_get "Color" (Variables|Default|GetColor) :!class /Script/Engine.MaterialInstanceDynamic))