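; Parent Blueprint for inspectable items that the player picks up, holds in front of the camera and releases.
; Interactwith toggles inspection through the player's CurrentItem and IsGrabbed, also switching the mesh's custom depth.
; StartInspection attaches to the player's Item component at InspectDistance along camera forward, disabling physics and collision; StopInspection detaches and restores both.
; Tick shows the E prompt while the empty-handed player looks at this actor.
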(event EventInteractwith
  (params (PlayerCharacter :type BP%20First%20Person%20Character%20Object%20Reference))
  (bind _output_get (Variables|Default|SetPlayer%20Character PlayerCharacter))
  (bind _currentitem (Variables|/Game/FirstPerson/Blueprints/BP_FirstPersonCharacter.BP_FirstPersonCharacter_C|GetCurrentItem _output_get)
    (:then
      (CallFunction|StopInspection _currentitem)
      (Variables|/Game/FirstPerson/Blueprints/BP_FirstPersonCharacter.BP_FirstPersonCharacter_C|SetCurrentItem _output_get 0)
      (Variables|/Game/FirstPerson/Blueprints/BP_FirstPersonCharacter.BP_FirstPersonCharacter_C|SetIsGrabbed _output_get false)
      (Rendering|SetRenderCustomDepth (Variables|Default|GetInspectMesh) true))
    (:else
      (CallFunction|StartInspection)
      (Variables|/Game/FirstPerson/Blueprints/BP_FirstPersonCharacter.BP_FirstPersonCharacter_C|SetIsGrabbed (Variables|Default|GetPlayer%20Character) true)
      (Rendering|SetVisibility (Variables|Default|GetE_Prompt_Widget) false false)
      (Rendering|SetRenderCustomDepth (Variables|Default|GetInspectMesh) false))))

(event EventTick
  (params (DeltaSeconds :type Float%20%28single-precision%29))
  (bind _asbp_first_person_character (Utilities|Casting|CastToBP_FirstPersonCharacter (Game|Player|GetPlayerPawn 0)))
  (if (not (Variables|/Game/FirstPerson/Blueprints/BP_FirstPersonCharacter.BP_FirstPersonCharacter_C|GetIsGrabbed _asbp_first_person_character))
    (if (== self (Variables|/Game/FirstPerson/Blueprints/BP_FirstPersonCharacter.BP_FirstPersonCharacter_C|GetLookAtActor _asbp_first_person_character))
      (Rendering|SetVisibility (Variables|Default|GetE_Prompt_Widget) true false)
      (else
        (Rendering|SetVisibility (Variables|Default|GetE_Prompt_Widget) false false)))))

(fn ConstructionScript)

(fn StartInspection
  (bind _returnvalue (Game|GetPlayerCameraManager 0))
  (bind _inspectmesh (Variables|Default|GetInspectMesh))
  (Input|EnableInput (Game|GetPlayerController 0))
  (Transformation|AttachComponentToComponent (Variables|/Game/FirstPerson/Blueprints/BP_FirstPersonCharacter.BP_FirstPersonCharacter_C|GetItem (Variables|Default|GetPlayer%20Character)) "None" "SnapToTarget" "KeepWorld" "KeepRelative" true)
  (Physics|SetSimulatePhysics _inspectmesh false)
  (Collision|SetCollisionEnabled _inspectmesh "NoCollision")
  (Variables|/Game/FirstPerson/Blueprints/BP_FirstPersonCharacter.BP_FirstPersonCharacter_C|SetCurrentItem (Variables|Default|GetPlayer%20Character) self)
  (Transformation|SetActorLocation (+ (Camera|GetCameraLocation _returnvalue) (* (Math|Vector|GetForwardVector (Camera|GetCameraRotation _returnvalue)) (Variables|Default|GetInspectDistance))) false false))

(fn StopInspection
  (bind _inspectmesh (Variables|Default|GetInspectMesh))
  (Transformation|DetachFromActor "KeepWorld" "KeepWorld" "KeepWorld")
  (Physics|SetSimulatePhysics _inspectmesh true)
  (Collision|SetCollisionEnabled _inspectmesh "QueryAndPhysics"))