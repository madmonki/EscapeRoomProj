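; BP_PictureFrame_Puzzle is an interactable picture frame puzzle piece that rotates a quarter turn per interaction.
; A timeline lerps the frame's pitch by 90 degrees with a sound, while a FrameMoving flag blocks overlapping turns.
; When each turn finishes, it saves the new rotation, advances a four-step position counter and prints a solved message if that position matches PuzzleAnswer.
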(event Custom|RotatePainting
  (if (not (Variables|Default|GetFrameMoving))
    (Variables|Default|SetFrameMoving true)
    (Audio|PlaySound2D "/Game/DoomsDayge/Sound/327555__damianminnie__moving-object-heavy-object-moved-accros-surface.327555__damianminnie__moving-object-heavy-object-moved-accros-surface" 1.0 1.0 0.0 0 0)
    (bind _rotation (Timeline|PaintingRotation PlayFromStart)
      (:Update
        (Transformation|SetRelativeRotation (Variables|Default|GetPictureFrame) (Math|Rotator|MakeRotator 0.0 (Math|Float|Lerp (.pitch (Variables|Default|GetStartingRotationFrame)) (+ (.pitch (Variables|Default|GetStartingRotationFrame)) 9e+01) _rotation) 0.0) false false))
      (:Finished
        (Variables|Default|SetStartingRotationFrame (Math|Rotator|MakeRotator 0.0 (Math|Float|Lerp (.pitch (Variables|Default|GetStartingRotationFrame)) (+ (.pitch (Variables|Default|GetStartingRotationFrame)) 9e+01) _rotation) 0.0))
        (Variables|Default|SetFrameMoving false)
        (bind _result (Math|Integer|IncrementInt (Variables|Default|GetFramePosition))
          (:%20%20
            (bind _output_get (Variables|Default|SetFramePosition (Math|Integer|%(Integer) _result 4)))
            (if (== _output_get (Variables|Default|GetPuzzleAnswer))
              (Development|PrintString "Puzzle Solved"))))))))

(event EventInteraction
  (CallFunction|RotatePainting))

(event EventBeginPlay
  (Variables|Default|SetStartingRotationFrame (Variables|/Script/Engine.SceneComponent|GetRelativeRotation (Variables|Default|GetPictureFrame))))

(fn ConstructionScript
  (|CallParentFunction))