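; BP_BookPick2 is a book pickup Blueprint, judging by its name, that adds an erratic spin to its InspectMesh.
; After running the parent Tick, it checks the Spin flag and, when set, nudges the mesh's relative roll, pitch and yaw toward small random offsets.
; Each axis is smoothed with FInterpTo, giving a random wobbling drift rather than a steady rotation.
; The construction script only calls its parent.
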(event EventBeginPlay
  (|CallParentFunction) ; This node is disabled and will not be called.\nDrag off pins to build functionality.
)

(event Collision|EventActorBeginOverlap
  (params (OtherActor :type Actor%20Object%20Reference))
  (|CallParentFunction OtherActor) ; This node is disabled and will not be called.\nDrag off pins to build functionality.
)

(event EventTick
  (params (DeltaSeconds :type Float%20%28single-precision%29))
  (bind _returnvalue (Math|Random|RandomFloatinRange -1e+01 1e+01))
  (bind _inspectmesh (Variables|Default|GetInspectMesh))
  (bind _relativerotation (Variables|/Script/Engine.SceneComponent|GetRelativeRotation _inspectmesh))
  (|CallParentFunction DeltaSeconds)
  (if (Variables|Default|GetSpin)
    (Transformation|SetRelativeRotation _inspectmesh (Math|Rotator|MakeRotator (Math|Interpolation|FInterpTo (.roll _relativerotation) (+ (.roll _relativerotation) _returnvalue) (Utilities|Time|GetWorldDeltaSeconds) 7.0) (Math|Interpolation|FInterpTo (.pitch _relativerotation) (+ (.pitch _relativerotation) _returnvalue) (Utilities|Time|GetWorldDeltaSeconds) 7.0) (Math|Interpolation|FInterpTo (.yaw _relativerotation) (+ (.yaw _relativerotation) _returnvalue) (Utilities|Time|GetWorldDeltaSeconds) 7.0)) false false)))

(fn ConstructionScript
  (|CallParentFunction))