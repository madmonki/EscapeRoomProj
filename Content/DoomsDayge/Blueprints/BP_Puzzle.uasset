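; BP_Puzzle builds a 3x3 tile puzzle with one blank space when play begins.
; A grid macro spawns upright-rotated BP_PuzzleTile actors around a hard-coded center, passing each its column, row and grid size, and collects them in PuzzleArray.
; After each spawn it rescans the array, flagging the seventh tile as blank and giving it the Xray material.
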(event EventBeginPlay
  (bind _returnvalue (Class|KismetSystemLibrary|MakeLiteralInteger 3))
  (bind (_current_point _total_points _0_1_phase _poly_center _x_row _y_row) (Utilities|2DGridExecutionMacro 51.0 "1400.000000,1400.000000,150.000000" _returnvalue _returnvalue)
    (:Per%20Poly%20Execution
      (bind _returnvalue_2 (Game|SpawnActorfromClass "/Game/DoomsDayge/Blueprints/BP_PuzzleTile.BP_PuzzleTile_C" (Math|Transform|MakeTransform _poly_center "0.000000,0.000000,90.000000" "1.000000,1.000000,1.000000") "Undefined" "MultiplyWithRoot" 0 _x_row _y_row _returnvalue 0))
      (Utilities|Array|Add (Variables|Default|GetPuzzle%20Array) _returnvalue_2)
      (for (_array_element _array_index) (Variables|Default|GetPuzzle%20Array)
        (if (== _array_index 6)
          (Variables|/Game/DoomsDayge/Blueprints/BP_PuzzleTile.BP_PuzzleTile_C|SetIsBlank _array_element true)
          (Rendering|Material|SetMaterial (Variables|/Game/DoomsDayge/Blueprints/BP_PuzzleTile.BP_PuzzleTile_C|GetCube _array_element) 0 "/Engine/VREditor/TransformGizmo/Xray.Xray"))))))

(fn ConstructionScript)